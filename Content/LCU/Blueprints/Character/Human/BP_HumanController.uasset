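; BP_HumanController is the controller for the human character, turning Enhanced Input into movement, camera, targeting, inventory and combat actions, with Tab toggling a pawn switch.
; Jump, equip and attacks request gameplay-tagged states from StateManager, with attacks trying Equip before attacking.
; Movement and attack inputs also pass through MakeBuffer, which records them in InputManager while its buffer is open.
; Mouse look is suppressed while the character's BaseCombat has a valid target.
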(event `self.ReceiveTick`
  (params (DeltaSeconds :type "Float (single-precision)")))

(event `Key|Tab`
  (params (Key :type "Key Structure"))
  ;[1 1 1] 빙의 스위칭
  (:`Pressed`
    (`self.TogglePawnChange`)))

(event `EnhancedInput|/Game/LCU/Blueprints/Character/Human/HumanEnhanced/HumanInput/IA_Human_MoveForward`
  (params (ActionValue :type "Float (double-precision)") (ElapsedSeconds :type "Float (double-precision)") (TriggeredSeconds :type "Float (double-precision)") (InputAction :type "InputAction Object Reference" :default "/Game/LCU/Blueprints/Character/Human/HumanEnhanced/HumanInput/IA_Human_MoveForward.IA_Human_MoveForward"))
  (bind _returnvalue (`self.K2_GetPawn`))
  (bind (_returnvalue_roll _returnvalue_pitch _returnvalue_yaw) (`KismetMathLibrary.BreakRotator` (`Pawn.GetControlRotation` _returnvalue)))
  ;[1 1 1] Move
  (:`Triggered`
    (`self.SetFwdBak` ActionValue)
    (`self.MakeBuffer` (struct :`TagName` "Input.MoveForWard") InputAction
      (:`Out`
        (`Pawn.AddMovementInput` _returnvalue (`KismetMathLibrary.GetForwardVector` (`KismetMathLibrary.MakeRotator` 0.0 0.0 _returnvalue_yaw)) (* (* ActionValue (`self.Speed`)) (`GameplayStatics.GetWorldDeltaSeconds`)) false)))))

(event `EnhancedInput|/Game/LCU/Blueprints/Character/Human/HumanEnhanced/HumanInput/IA_Human_Turn`
  (params (ActionValue :type "Float (double-precision)") (ElapsedSeconds :type "Float (double-precision)") (TriggeredSeconds :type "Float (double-precision)") (InputAction :type "InputAction Object Reference" :default "/Game/LCU/Blueprints/Character/Human/HumanEnhanced/HumanInput/IA_Human_Turn.IA_Human_Turn"))
  ;[1 1 1] 마우스 움직임 나중에 포커싱을 추가하면 바뀔것이다
  (:`Triggered`
    (bind _asbp_human_character (cast `/Game/LCU/Blueprints/Character/Human/BP_HumanCharacter` (`self.K2_GetPawn`))
      (:`then`
        (if (not (`KismetSystemLibrary.IsValid` (`BaseCombatComponent.TargetActor` (`/Game/LCU/Blueprints/Character/Human/BP_HumanCharacter.BaseCombat` _asbp_human_character))))
          (`Pawn.AddControllerYawInput` (`self.K2_GetPawn`) (`KismetMathLibrary.FClamp` ActionValue -3.0 3.0) :!label _label)))
      (:`CastFailed`
        (goto _label)))))

(event `EnhancedInput|/Game/LCU/Blueprints/Character/Human/HumanEnhanced/HumanInput/IA_Human_LookUp`
  (params (ActionValue :type "Float (double-precision)") (ElapsedSeconds :type "Float (double-precision)") (TriggeredSeconds :type "Float (double-precision)") (InputAction :type "InputAction Object Reference" :default "/Game/LCU/Blueprints/Character/Human/HumanEnhanced/HumanInput/IA_Human_LookUp.IA_Human_LookUp"))
  ;[1 1 1] 마우스 움직임 나중에 포커싱을 추가하면 바뀔것이다
  (:`Triggered`
    (bind _asbp_human_character (cast `/Game/LCU/Blueprints/Character/Human/BP_HumanCharacter` (`self.K2_GetPawn`))
      (:`then`
        (if (not (`KismetSystemLibrary.IsValid` (`BaseCombatComponent.TargetActor` (`/Game/LCU/Blueprints/Character/Human/BP_HumanCharacter.BaseCombat` _asbp_human_character))))
          (`Pawn.AddControllerPitchInput` (`self.K2_GetPawn`) (`KismetMathLibrary.FClamp` ActionValue -3.0 3.0) :!label _label_2)))
      (:`CastFailed`
        (goto _label_2)))))

(event `EnhancedInput|/Game/LCU/Blueprints/Character/Human/HumanEnhanced/HumanInput/IA_Human_MoveRight`
  (params (ActionValue :type "Float (double-precision)") (ElapsedSeconds :type "Float (double-precision)") (TriggeredSeconds :type "Float (double-precision)") (InputAction :type "InputAction Object Reference" :default "/Game/LCU/Blueprints/Character/Human/HumanEnhanced/HumanInput/IA_Human_MoveRight.IA_Human_MoveRight"))
  (bind _returnvalue (`self.K2_GetPawn`))
  (bind (_returnvalue_roll _returnvalue_pitch _returnvalue_yaw) (`KismetMathLibrary.BreakRotator` (`Pawn.GetControlRotation` _returnvalue)))
  ;[1 1 1] Move
  (:`Triggered`
    (set `self.Direction` ActionValue)
    (`self.MakeBuffer` (struct :`TagName` "Input.MoveRight") InputAction
      (:`Out`
        (`Pawn.AddMovementInput` _returnvalue (`KismetMathLibrary.GetRightVector` (`KismetMathLibrary.MakeRotator` _returnvalue_roll 0.0 _returnvalue_yaw)) (* (* ActionValue (`self.Speed`)) (`GameplayStatics.GetWorldDeltaSeconds`)) false))))
  (:`Canceled`
    (set `self.Direction` ActionValue :!label _label_3))
  (:`Completed`
    (goto _label_3)))

(event `EnhancedInput|/Game/LCU/Blueprints/Character/Human/HumanEnhanced/HumanInput/IA_Human_Target`
  (params (ActionValue :type Boolean) (ElapsedSeconds :type "Float (double-precision)") (TriggeredSeconds :type "Float (double-precision)") (InputAction :type "InputAction Object Reference" :default "/Game/LCU/Blueprints/Character/Human/HumanEnhanced/HumanInput/IA_Human_Target.IA_Human_Target"))
  ;[1 1 1] 타겟팅
  (:`Started`
    (bind _asbp_human_character (cast `/Game/LCU/Blueprints/Character/Human/BP_HumanCharacter` (`self.K2_GetPawn`)))
    (`/Engine/EditorBlueprintResources/StandardMacros.IsValid` _asbp_human_character
      (:`Is Valid`
        (`BaseCombatComponent.SearchTargetActor` (`/Game/LCU/Blueprints/Character/Human/BP_HumanCharacter.BaseCombat` _asbp_human_character))))))

(event `EnhancedInput|/Game/LCU/Blueprints/Character/Human/HumanEnhanced/HumanInput/IA_Human_Jump`
  (params (ActionValue :type Boolean) (ElapsedSeconds :type "Float (double-precision)") (TriggeredSeconds :type "Float (double-precision)") (InputAction :type "InputAction Object Reference" :default "/Game/LCU/Blueprints/Character/Human/HumanEnhanced/HumanInput/IA_Human_Jump.IA_Human_Jump"))
  (bind _statemanager (`self.StateManager`))
  ;[1 1 1] 점프
  (:`Started`
    (`BaseStateManagerComponent.TryChangeStateOfClass` _statemanager (`GameplayStatics.GetObjectClass` (`BaseStateManagerComponent.GetStateOfGameplayTag` _statemanager (struct :`TagName` "State.Jump"))) true (struct))))

(event `EnhancedInput|/Game/LCU/Blueprints/Character/Human/HumanEnhanced/HumanInput/IA_Human_EquipUnEquip`
  (params (ActionValue :type Boolean) (ElapsedSeconds :type "Float (double-precision)") (TriggeredSeconds :type "Float (double-precision)") (InputAction :type "InputAction Object Reference" :default "/Game/LCU/Blueprints/Character/Human/HumanEnhanced/HumanInput/IA_Human_EquipUnEquip.IA_Human_EquipUnEquip"))
  (bind _statemanager (`self.StateManager`))
  ;[1 1 1] 장착, 장착 해제
  (:`Started`
    (`BaseStateManagerComponent.TryChangeStatesOfClass` _statemanager (`|MakeArray` (`GameplayStatics.GetObjectClass` (`BaseStateManagerComponent.GetStateOfGameplayTag` _statemanager (struct :`TagName` "State.Equip"))) (`GameplayStatics.GetObjectClass` (`BaseStateManagerComponent.GetStateOfGameplayTag` _statemanager (struct :`TagName` "State.UnEquip")))) true)))

(event `EnhancedInput|/Game/LCU/Blueprints/Character/Human/HumanEnhanced/HumanInput/IA_Human_Inventory`
  (params (ActionValue :type Boolean) (ElapsedSeconds :type "Float (double-precision)") (TriggeredSeconds :type "Float (double-precision)") (InputAction :type "InputAction Object Reference" :default "/Game/LCU/Blueprints/Character/Human/HumanEnhanced/HumanInput/IA_Human_Inventory.IA_Human_Inventory"))
  (bind _returnvalue (`GameplayStatics.GetPlayerController` 0))
  (:`Started`
    (bind _returnvalue_2 (`|CreateWidget` "/Game/JEP/UI/WB_PlayerInventory.WB_PlayerInventory_C"))
    (`UserWidget.AddToViewport` _returnvalue_2 0)
    (`WidgetBlueprintLibrary.SetInputMode_UIOnlyEx` _returnvalue _returnvalue_2)
    (set `PlayerController.bShowMouseCursor` true _returnvalue)))

(event `EnhancedInput|/Game/LCU/Blueprints/Character/Human/HumanEnhanced/HumanInput/IA_Human_SpecialAttack`
  (params (ActionValue :type Boolean) (ElapsedSeconds :type "Float (double-precision)") (TriggeredSeconds :type "Float (double-precision)") (InputAction :type "InputAction Object Reference" :default "/Game/LCU/Blueprints/Character/Human/HumanEnhanced/HumanInput/IA_Human_SpecialAttack.IA_Human_SpecialAttack"))
  ;[1 1 1] 차징공격
  (:`Started`
    (`self.MakeBuffer` (struct :`TagName` "Input.AttackCharging") InputAction
      (:`Out`
        (bind _returnvalue (`BaseStateManagerComponent.TryChangeStateOfTag` (`self.StateManager`) (struct :`TagName` "State.Equip") true (struct)))
        (if (not _returnvalue)
          (`BaseStateManagerComponent.TryChangeStateOfTag` (`self.StateManager`) (struct :`TagName` "State.AttackCharge") true (struct))))))
  (:`Canceled`
    (`self.MakeBuffer` (struct :`TagName` "Input.SpecialAttack") InputAction :!label _label_4))
  (:`Completed`
    (goto _label_4)))

(event `EnhancedInput|/Game/LCU/Blueprints/Character/Human/HumanEnhanced/HumanInput/IA_Human_NormalAttack`
  (params (ActionValue :type Boolean) (ElapsedSeconds :type "Float (double-precision)") (TriggeredSeconds :type "Float (double-precision)") (InputAction :type "InputAction Object Reference" :default "/Game/LCU/Blueprints/Character/Human/HumanEnhanced/HumanInput/IA_Human_NormalAttack.IA_Human_NormalAttack"))
  (bind _statemanager (`self.StateManager`))
  ;[1 1 1] 기본 콤보 공격
  (:`Started`
    (`self.MakeBuffer` (struct :`TagName` "Input.NorMalAttack") InputAction
      (:`Out`
        (bind _returnvalue (`BaseStateManagerComponent.TryChangeStateOfTag` (`self.StateManager`) (struct :`TagName` "State.Equip") true (struct)))
        (if (not _returnvalue)
          (set `BaseStateManagerComponent.bIsSpecialAttack` false _statemanager)
          (`BaseStateManagerComponent.TryChangeStateOfTag` _statemanager (struct :`TagName` "State.Attack") true (struct :`TagName` "Ability.Attack.NormalAttack")))))))

(event `EnhancedInput|/Game/LCU/Blueprints/Character/Human/HumanEnhanced/HumanInput/IA_Human_UltimateAttack`
  (params (ActionValue :type Boolean) (ElapsedSeconds :type "Float (double-precision)") (TriggeredSeconds :type "Float (double-precision)") (InputAction :type "InputAction Object Reference" :default "/Game/LCU/Blueprints/Character/Human/HumanEnhanced/HumanInput/IA_Human_UltimateAttack.IA_Human_UltimateAttack"))
  (:`Triggered`
    (`self.MakeBuffer` (struct :`TagName` "Input.UltimateAttack") InputAction
      (:`Out`
        (bind _returnvalue (`BaseStateManagerComponent.TryChangeStateOfTag` (`self.StateManager`) (struct :`TagName` "State.Equip") true (struct)))
        (if (not _returnvalue)
          (`BaseStateManagerComponent.TryChangeStateOfTag` (`self.StateManager`) (struct :`TagName` "State.Attack") true (struct :`TagName` "Ability.Attack.UltimateAttack")))))))

(fn `InitController`
  (bind _statemanager (`self.StateManager`))
  (`BaseStateManagerComponent.ClearStatesComponent` _statemanager)
  (`BaseStateManagerComponent.InitializeStateManagerComponent` _statemanager (`self.K2_GetPawn`)))

(fn `UserConstructionScript`)