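; BP_Fist is the fist melee weapon for human characters, damaging BaseEnemy actors while attacking is enabled.
; SetAttackable toggles a flag that makes Tick run a multi-sphere trace forward from the attack socket on the owner's mesh, found through WeaponManager.
; Each enemy hit takes AttackStat damage and is recorded in EnemyActors to prevent repeat hits; this graph never clears that list.
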(event `self.ReceiveTick`
  (params (DeltaSeconds :type "Float (single-precision)"))
  (bind (_returnvalue_location _returnvalue_rotation) (`KismetMathLibrary.BreakTransform` (`SceneComponent.GetSocketTransform` (`Character.Mesh` (`WeaponComponent.OwnerCharacter` (`self.WeaponManager`))) (`self.AttackSocket`) "RTS_World")))
  (`parent.ReceiveTick` DeltaSeconds)
  (if (`self.bAttackable`)
    (bind _outhits (`KismetSystemLibrary.SphereTraceMulti` :`Start` _returnvalue_location :`End` (+ _returnvalue_location (* (`KismetMathLibrary.GetForwardVector` _returnvalue_rotation) (`self.TraceLength`))) :`Radius` 20.0 :`TraceChannel` "TraceTypeQuery3" :`DrawTime` 1.0))
    (for _array_element _outhits
      (bind _asbase_enemy (cast `BaseEnemy` (`.HitActor` (`GameplayStatics.BreakHitResult` _array_element))))
      (if (not (`KismetArrayLibrary.Array_Contains` (`self.EnemyActors`) _asbase_enemy))
        (`GameplayStatics.ApplyDamage` _asbase_enemy (`self.AttackStat`))
        (`KismetArrayLibrary.Array_AddUnique` (`self.EnemyActors`) _asbase_enemy)))))

(event `/Game/LCH/Blueprints/Character/Character/BPI_Equipable.SetAttackable`
  (params (bAttackable :type Boolean))
  (set `self.bAttackable` bAttackable))

(fn `UserConstructionScript`)