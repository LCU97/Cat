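; BP_HumanCharacter is the human character Blueprint, which sets up its gameplay components and HUD when play begins.
; Once its BP_HumanController is confirmed, BeginPlay initializes the controller, ability manager, weapon, camera manager and combat components, passing in-game and ultimate cameras where needed, then creates the character UI.
; AnyDamage lowers health with a floor at zero and has no death handling.
; The construction script assigns groom assets and bindings for hair and eyebrows.
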(event `self.ReceiveBeginPlay`
  (bind _asbp_human_controller (cast `/Game/LCU/Blueprints/Character/Human/BP_HumanController` (`self.GetController`)))
  (`/Engine/EditorBlueprintResources/StandardMacros.IsValid` _asbp_human_controller
    (:`Is Valid`
      (`/Game/LCU/Blueprints/Character/Human/BP_HumanController.InitController` _asbp_human_controller)
      (`BaseAbilityManagerComponent.InitializeAbilityManager` (`self.BaseAbilityManager`))
      (`WeaponComponent.InitWeaponComponent` (`self.Weapon`))
      (`CameraManagerComponent.InitCameraManager` (`self.CameraManager`) (`self.InGameCamera`) (`self.UltimateCamera`))
      (`BaseCombatComponent.InitCombatComponent` (`self.BaseCombat`) (`self.InGameCamera`))
      (bind _returnvalue (`|CreateWidget` "/Game/LCU/Blueprints/Widget/WBP_CharacterUI.WBP_CharacterUI_C" (`GameplayStatics.GetPlayerController` 0)))
      (`UserWidget.AddToViewport` _returnvalue 0))))

(event `self.ReceiveTick`
  (params (DeltaSeconds :type "Float (single-precision)")))

(event `self.ReceiveAnyDamage`
  (params (Damage :type "Float (single-precision)") (DamageType :type "DamageType Object Reference") (InstigatedBy :type "Controller Object Reference") (DamageCauser :type "Actor Object Reference"))
  (set `self.CurrentHealth` (- (`self.CurrentHealth`) Damage))
  (if (<= (`self.CurrentHealth`) 0.0)
    (set `self.CurrentHealth` 0.0)))

(fn `UserConstructionScript`
  (bind _hairgroom (`self.HairGroom`))
  (bind _eye (`self.Eye`))
  (`GroomComponent.SetGroomAsset` _hairgroom "/Game/EchoContent/Characters/Echo/Hair/Hair_S_UpdoBuns.Hair_S_UpdoBuns")
  (`GroomComponent.SetBindingAsset` _hairgroom "/Game/EchoContent/Characters/Echo/Hair/Hair_S_UpdoBuns_Echo_M3D_LOD0_Binding.Hair_S_UpdoBuns_Echo_M3D_LOD0_Binding")
  (`GroomComponent.SetGroomAsset` _eye "/Game/EchoContent/Characters/Echo/Hair/Eyebrows_L_Echo.Eyebrows_L_Echo")
  (`GroomComponent.SetBindingAsset` _eye "/Game/EchoContent/Characters/Echo/Hair/Eyebrows_L_Echo_Echo_M3D_LOD0_Binding.Eyebrows_L_Echo_Echo_M3D_LOD0_Binding"))