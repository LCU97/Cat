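; Normal monster AI character that chases and attacks the player, with a health bar turned toward the camera every Tick.
; ChasePlayer moves to the player, triggers the attack montage on success, then repeats after a delay; montage end fires OnAttackEnd.
; It exposes a patrol spline and sets walk speed from a movement state.
; Damage is only printed; hit reaction and health bar widget cast are unconnected.
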(event `self.ReceiveBeginPlay`)

(event `self.ReceiveTick`
  (params (DeltaSeconds :type "Float (single-precision)"))
  (bind _healthbar (`self.HealthBar`))
  (`SceneComponent.K2_SetWorldRotation` _healthbar (`KismetMathLibrary.FindLookAtRotation` (`SceneComponent.K2_GetComponentLocation` _healthbar) (`SceneComponent.K2_GetComponentLocation` (`PlayerCameraManager.TransformComponent` (`GameplayStatics.GetPlayerCameraManager` 0)))) false false))

(event `ChasePlayer`
  (`|AIMoveTo` self (0.0 0.0 0.0) (`GameplayStatics.GetPlayerCharacter` 0) 150.0
    (:`OnSuccess`
      (`self.Attacking`)
      (`KismetSystemLibrary.Delay` 1.0)
      (`self.ChasePlayer`))))

(event `Attacking`
  (`|PlayMontage` (`self.Mesh`) "/Game/LCU/Blueprints/Character/AI/Animation/NormalMonster_Attack_Montage.NormalMonster_Attack_Montage"
    (:`OnCompleted`
      _)
    (:`OnBlendOut`
      _)
    (:`OnInterrupted`
      _))
  (`self.OnAttackEnd`))

(event `self.ReceiveAnyDamage`
  (params (Damage :type "Float (single-precision)") (DamageType :type "DamageType Object Reference") (InstigatedBy :type "Controller Object Reference") (DamageCauser :type "Actor Object Reference"))
  (`KismetSystemLibrary.PrintString` (`KismetStringLibrary.Conv_DoubleToString` Damage)))

(fn `GetPatrolSpline`
  (returns (PatrolSpline :type "/Game/LCU/Blueprints/Character/AI/BP_LCU_Patrol Object Reference"))
  (return (`self.PatrolSpline`)))

(fn `SetMovementSpeed`
  (params (Speed :type "/Game/LCU/Blueprints/Character/AI/E_LCU_MovementSpeed Enum" :default "NewEnumerator0"))
  (returns (SpeedValue :type "Float (double-precision)"))
  (bind _output_get (set `CharacterMovementComponent.MaxWalkSpeed` (select `/Game/LCU/Blueprints/Character/AI/E_LCU_MovementSpeed` Speed :`NewEnumerator1` 100.0 :`NewEnumerator2` 300.0 :!type "Float (single-precision)") (`self.CharacterMovement`)))
  (return _output_get))

(fn `UserConstructionScript`)