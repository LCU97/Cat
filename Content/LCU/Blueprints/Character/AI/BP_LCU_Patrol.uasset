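; BP_LCU_Patrol is an AI patrol route actor that tracks a current point along its PatrolSpline.
; IncrementPatrol steps PatrolIndex by PatrolDirection and flips the direction at the first and last spline points, producing a ping-pong route.
; GetSplinePointWorld returns the current point's location, though it queries the spline in Local space despite its name.
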(event `IncrementPatrol`
  (bind _output_get (set `self.PatrolIndex` (+ (`self.PatrolIndex`) (`self.PatrolDirection`))))
  (if (== _output_get (- (`SplineComponent.GetNumberOfSplinePoints` (`self.PatrolSpline`)) 1))
    (set `self.PatrolDirection` -1)
    (elif (== (`self.PatrolIndex`) 0)
      (set `self.PatrolDirection` 1))))

(fn `GetSplinePointWorld`
  (returns (Vec :type "Vector Structure"))
  (return (`SplineComponent.GetLocationAtSplinePoint` (`self.PatrolSpline`) (`self.PatrolIndex`) "Local")))

(fn `UserConstructionScript`)