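; Player cat character Blueprint that can pull the human character to itself and be shown or hidden.
; Pressing C finds the LCH_BP_HumanCharacter_Child actor and moves it, without sweep, to a point slightly above and in front of the cat.
; HiddenCat and ShowCat set the Possess flag alongside the mesh's in-game visibility; BeginPlay, overlap and Tick events are empty.
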(event `Key|C`
  (params (Key :type "Key Structure"))
  (bind (_returnvalue_x _returnvalue_y _returnvalue_z) (`KismetMathLibrary.BreakVector` (`self.K2_GetActorLocation`)))
  (:`Pressed`
    (bind _returnvalue (`GameplayStatics.GetActorOfClass` "/Game/LCH/Blueprints/Character/Character/LCH_BP_HumanCharacter_Child.LCH_BP_HumanCharacter_Child_C"))
    (`/Engine/EditorBlueprintResources/StandardMacros.IsValid` _returnvalue
      (:`Is Valid`
        (`self.K2_SetActorLocation` _returnvalue (+ (`KismetMathLibrary.MakeVector` _returnvalue_x _returnvalue_y (+ _returnvalue_z 70.0)) (* (`self.GetActorForwardVector`) 80.0)) false false)))))

(fn `HiddenCat`
  (set `self.bPossess` false)
  (`SceneComponent.SetHiddenInGame` (`self.Mesh`) true false))

(fn `ShowCat`
  (set `self.bPossess` true)
  (`SceneComponent.SetHiddenInGame` (`self.Mesh`) false false))

(fn `UserConstructionScript`)