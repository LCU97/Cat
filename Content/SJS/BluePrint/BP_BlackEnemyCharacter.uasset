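; BP_BlackEnemyCharacter is an enemy character Blueprint that plays montage-driven attacks.
; Attack plays one of three random attack montages.
; Attack2 checks distance to the player: up close it chains a random back or side roll into a paired attack, otherwise a forward roll into a fixed attack.
; Each sequence fires its attack-end dispatcher whether the final montage completes or is interrupted.
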(event `self.ReceiveTick`
  (params (DeltaSeconds :type "Float (single-precision)")))

(event `Attack`
  (`|PlayMontage` (`self.Mesh`) (select `int` (`KismetMathLibrary.RandomInteger` 3) :`0` "/Game/SJS/EnemyAnimations/Anim_Attack_2_MontageAtackKick.Anim_Attack_2_MontageAtackKick" :`1` "/Game/SJS/EnemyAnimations/Anim_Attack_4_MontageKnife2.Anim_Attack_4_MontageKnife2" :`2` "/Game/SJS/EnemyAnimations/Anim_Attack_5_Montage.Anim_Attack_5_Montage" :!type "AnimMontage Object Reference")
    (:`OnCompleted`
      _)
    (:`OnInterrupted`
      _))
  (`self.BlackOnAttackEnd`))

(event `Attack2`
  (bind _mesh (`self.Mesh`))
  (bind _mesh_2 (`self.Mesh`))
  (bind _output_get (set `self.distance` (`KismetMathLibrary.Vector_Distance` (`self.K2_GetActorLocation` (`PawnMovementComponent.GetPawnOwner` (`self.CharacterMovement`))) (`self.K2_GetActorLocation` (`GameplayStatics.GetPlayerPawn` 0)))))
  (if (< _output_get 200.0)
    (bind _output_get_2 (set `self.RandomValue` (`KismetMathLibrary.RandomInteger` 3)))
    (`|PlayMontage` _mesh (select `int` _output_get_2 :`0` "/Game/SJS/EnemyAnimations/Anim_Roll_Bwd_Montage.Anim_Roll_Bwd_Montage" :`1` "/Game/SJS/EnemyAnimations/Anim_Roll_Lt_Montage.Anim_Roll_Lt_Montage" :`2` "/Game/SJS/EnemyAnimations/Anim_Roll_Rt_Montage.Anim_Roll_Rt_Montage" :!type "AnimMontage Object Reference")
      (:`OnCompleted`
        _)
      (:`OnInterrupted`
        _))
    (`|PlayMontage` _mesh (select `int` _output_get_2 :`0` "/Game/SJS/EnemyAnimations/Anim_Attack_7_Montage.Anim_Attack_7_Montage" :`1` "/Game/SJS/EnemyAnimations/Anim_Attack_5_Montage.Anim_Attack_5_Montage" :`2` "/Game/SJS/EnemyAnimations/Anim_Attack_4_MontageKnife2.Anim_Attack_4_MontageKnife2" :!type "AnimMontage Object Reference")
      (:`OnCompleted`
        _)
      (:`OnInterrupted`
        _))
    (`self.BlackOnAttackEnd2`)
    (else
      (`|PlayMontage` _mesh_2 "/Game/SJS/EnemyAnimations/Anim_Roll_Fwd_Montage.Anim_Roll_Fwd_Montage"
        (:`OnCompleted`
          _)
        (:`OnInterrupted`
          _))
      (`|PlayMontage` _mesh_2 "/Game/SJS/EnemyAnimations/Anim_Attack_6_Montage.Anim_Attack_6_Montage"
        (:`OnCompleted`
          _)
        (:`OnInterrupted`
          _))
      (`self.BlackOnAttackEnd2`))))

(fn `UserConstructionScript`)