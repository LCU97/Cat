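; BP_WhiteTiger is a white tiger character that chases the first player pawn and plays an attack animation on reaching it.
; On BeginPlay it starts an AI MoveTo loop that, on success, prints a debug message, calls Attack1, waits briefly and follows again.
; Attack1 starts the same cat attack montage through both PlayAnimMontage and PlayMontage, with no damage logic.
; A failed move is unhandled, so the loop stops there.
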(event `self.ReceiveBeginPlay`
  (`self.FollowPlayer`))

(event `self.ReceiveTick`
  (params (DeltaSeconds :type "Float (single-precision)")))

(event `FollowPlayer`
  (`|AIMoveTo` self (0.0 0.0 0.0) (`GameplayStatics.GetPlayerPawn` 0) 100.0
    (:`OnSuccess`
      (`KismetSystemLibrary.PrintString` "Hello")
      (`self.Attack1`)
      (`KismetSystemLibrary.Delay` 2.0)
      (`self.FollowPlayer`))))

(event `Attack1`
  (`self.PlayAnimMontage` "/Game/LCH/Blueprints/Character/Cats/Animations/AM_Anim_CatStray_Attack_F.AM_Anim_CatStray_Attack_F")
  (`|PlayMontage` (`self.Mesh`) "/Game/LCH/Blueprints/Character/Cats/Animations/AM_Anim_CatStray_Attack_F.AM_Anim_CatStray_Attack_F"))

(fn `UserConstructionScript`)