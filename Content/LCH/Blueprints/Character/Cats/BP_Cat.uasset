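; Cat companion NPC that stays put until its dialogue finishes, then follows the player.
; TriggerZone shows the dialog widget and Talk steps through lines, finally setting the player's IsCat and enabling walk speed for the looping AIMoveTo.
; Attack1 spawns a collisionless white tiger, driving its forward motion and opacity by Timeline during the attack montage, then destroys it.
; HiddenAICat and ShowAICat toggle mesh visibility and both set Possess true.
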(event `self.ReceiveBeginPlay`
  (`self.FollowPlayer`)
  (set `CharacterMovementComponent.MaxWalkSpeed` 0.0 (`self.CharacterMovement`)))

(event `self.ReceiveTick`
  (params (DeltaSeconds :type "Float (single-precision)")))

(event `FollowPlayer`
  (`|AIMoveTo` self (0.0 0.0 0.0) (`GameplayStatics.GetPlayerPawn` 0) 100.0
    (:`then`
      (`KismetSystemLibrary.Delay` 2.0)
      (`self.FollowPlayer`))))

(event `Attack1`
  (bind _returnvalue (`|SpawnActorFromClass` "/Game/LCH/Blueprints/Character/Tiger/BP_WhiteTiger.BP_WhiteTiger_C" (`KismetMathLibrary.MakeTransform` (- (- (`self.K2_GetActorLocation`) (* (`self.GetActorForwardVector`) 200.0)) (* (`self.GetActorUpVector`) 200.0)) (`self.K2_GetActorRotation`)) "AdjustIfPossibleButAlwaysSpawn" "MultiplyWithRoot" self null))
  (bind _capsulecomponent (`Character.CapsuleComponent` _returnvalue))
  (`PrimitiveComponent.SetSimulatePhysics` _capsulecomponent false)
  (`PrimitiveComponent.SetCollisionEnabled` _capsulecomponent "NoCollision")
  (bind _returnvalue_2 (`PrimitiveComponent.CreateDynamicMaterialInstance` (`Character.Mesh` _returnvalue) 0 "/Game/LCH/Blueprints/Character/Tiger/Materials/M_WhiteTiger.M_WhiteTiger" "None"))
  (`self.PlayAnimMontage` _returnvalue "/Game/LCH/Blueprints/Character/Tiger/Animations/AM_Anim_CatStray_Attack_F_Montage.AM_Anim_CatStray_Attack_F_Montage" 1.0 "None")
  (`|PlayMontage` (`self.Mesh`) "/Game/LCH/Blueprints/Character/Cats/Animations/AM_Anim_CatStray_Attack_F.AM_Anim_CatStray_Attack_F"
    (:`then`
      (bind (_direction _speed _opacity) (`Timeline|Timeline` :!via `PlayFromStart`)
        (:`Update`
          (`/Engine/EditorBlueprintResources/StandardMacros.IsValid` _returnvalue
            (:`Is Valid`
              (`self.K2_SetActorLocation` _returnvalue (+ (`self.K2_GetActorLocation` _returnvalue) (* (`self.GetActorForwardVector` _returnvalue) (* (`KismetMathLibrary.Lerp` 0.0 1000.0 _speed) (`GameplayStatics.GetWorldDeltaSeconds`)))) false false)
              (`MaterialInstanceDynamic.SetScalarParameterValue` _returnvalue_2 "OpacityMultiply" (`KismetMathLibrary.Lerp` 0.0 1.0 _opacity)))))))
    (:`OnCompleted`
      (`self.K2_DestroyActor` _returnvalue))))

(event `/Game/JEP/Blueprints/BPI_Dialogue.Talk`
  (if (not (`/Game/LCU/Blueprints/Character/Human/BP_HumanCharacter.IsCat` (cast `/Game/LCH/Blueprints/Character/Character/LCH_BP_HumanCharacter_Child` (`GameplayStatics.GetPlayerCharacter` 0) :!pure true)))
    (`/Engine/EditorBlueprintResources/StandardMacros.IncrementInt` (`self.DialogueIndex`)
      (:`  `
        (if (< (`self.DialogueIndex`) (`KismetArrayLibrary.Array_Length` (`self.Dialogue`)))
          (`self.UI`
            (:`then`
              _)
            (:`else`
              (bind _returnvalue (`|CreateWidget` "/Game/JEP/UI/WB_Dialog.WB_Dialog_C" (`GameplayStatics.GetPlayerController` 0)))
              (bind _output_get (set `self.UI` _returnvalue))
              (`UserWidget.AddToViewport` _output_get 0)))
          (`TextBlock.SetText` (`/Game/JEP/UI/WB_Dialog.Dialogue` (`self.UI`)) (`KismetTextLibrary.Conv_StringToText` (`|GetArrayItem` (`self.Dialogue`) (`self.DialogueIndex`))))
          (else
            (`Widget.RemoveFromParent` (`self.UI`))
            (set `/Game/LCH/Blueprints/Character/Character/LCH_BP_HumanCharacter_Child.IsCat` true (cast `/Game/LCH/Blueprints/Character/Character/LCH_BP_HumanCharacter_Child` (`GameplayStatics.GetPlayerCharacter` 0) :!pure true))
            (set `CharacterMovementComponent.MaxWalkSpeed` 500.0 (`self.CharacterMovement`))))))))

(event `self.TriggerZone.OnComponentBeginOverlap`
  (params (OverlappedComponent :type "PrimitiveComponent Object Reference") (OtherActor :type "Actor Object Reference") (OtherComp :type "PrimitiveComponent Object Reference") (OtherBodyIndex :type Integer) (bFromSweep :type Boolean) (SweepResult :type "HitResult Structure (by ref)"))
  (if (`/Game/LCU/Blueprints/Character/Human/BP_HumanCharacter.IsCat` (cast `/Game/LCH/Blueprints/Character/Character/LCH_BP_HumanCharacter_Child` (`GameplayStatics.GetPlayerCharacter` 0) :!pure true))
    (`Widget.RemoveFromParent` (`self.UI`))
    (else
      (bind _returnvalue (`|CreateWidget` "/Game/JEP/UI/WB_Dialog.WB_Dialog_C" (`GameplayStatics.GetPlayerController` 0)))
      (bind _output_get (set `self.UI` _returnvalue))
      (`UserWidget.AddToViewport` _output_get 0))))

(fn `HiddenAICat`
  (set `self.bPossess` true)
  (`SceneComponent.SetHiddenInGame` (`self.Mesh`) true false))

(fn `ShowAICat`
  (set `self.bPossess` true)
  (`SceneComponent.SetHiddenInGame` (`self.Mesh`) false false))

(fn `UserConstructionScript`)