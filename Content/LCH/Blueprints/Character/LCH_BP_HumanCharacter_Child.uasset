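; Child human character Blueprint that carries a cat on its back.
; On BeginPlay it runs the parent logic, then spawns a BP_CatOnTheBack at its own location and attaches it to the mesh's Cat_Socket, snapping location, rotation and scale.
; Overlap and Tick events are disabled stubs, and the construction script only calls the parent.
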(event `self.ReceiveBeginPlay`
  (`parent.ReceiveBeginPlay`)
  (bind _returnvalue (`|SpawnActorFromClass` "/Game/LCH/Blueprints/Character/BP_CatOnTheBack.BP_CatOnTheBack_C" (`KismetMathLibrary.Conv_VectorToTransform` (`self.K2_GetActorLocation`)) "AlwaysSpawn" "MultiplyWithRoot" null null))
  (`self.K2_AttachToComponent` _returnvalue (`self.Mesh`) "Cat_Socket" "SnapToTarget" "SnapToTarget" "SnapToTarget" true))

(fn `UserConstructionScript`
  (`parent.UserConstructionScript`))