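; Black Tiger enemy character with bite, claw, beam, fireball and monster-summon attacks, plus an HP widget.
; Each attack event plays a montage; all but fireball report back through CallOnAttackEnd.
; The beam chains Niagara finish callbacks from energy charge to beam and shockwave before ending.
; Patrol spline and speed helpers support movement, head hits trigger physical-animation reactions, and a Behavior Tree replaces the disconnected follow logic.
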(event `self.ReceiveBeginPlay`)

(event `ShowHealthUI`
  (bind _returnvalue (`|CreateWidget` "/Game/LCH/Blueprints/Character/Tiger/UI/LCH_WBP_TigerHPUI.LCH_WBP_TigerHPUI_C"))
  (`UserWidget.AddToViewport` _returnvalue 0))

(event `FollowPlayer`
  ;[1 1 1] Follow Player using 'AI Move To'
)

(event `BiteAttack`
  ;[1 1 1] Bite Attack
  (`|PlayMontage` (`self.Mesh`) "/Game/LCH/Blueprints/Character/Tiger/Animations/AM_ANIM_Lion_Bite_Montage.AM_ANIM_Lion_Bite_Montage"
    (:`OnCompleted`
      _)
    (:`OnBlendOut`
      _)
    (:`OnInterrupted`
      _))
  (`self.OnAttackEnd`))

(event `ClawsAttack`
  ;[1 1 1] ClawsAttack
  (`|PlayMontage` (`self.Mesh`) "/Game/LCH/Blueprints/Character/Tiger/Animations/ANIM_Lion_ClawsAttack_Montage.ANIM_Lion_ClawsAttack_Montage"
    (:`OnCompleted`
      _)
    (:`OnBlendOut`
      _)
    (:`OnInterrupted`
      _))
  (`self.OnAttackEnd`))

(event `BeamAttack`
  (params (BeamLocation :type "Vector Structure"))
  ;[1 1 1] Beam Attack
  (`|PlayMontage` (`self.Mesh`) "/Game/LCH/Blueprints/Character/Tiger/Animations/ANIM_Lion_Roar_Montage.ANIM_Lion_Roar_Montage"
    (:`then`
      (bind _returnvalue (`NiagaraFunctionLibrary.SpawnSystemAtLocation` "/Game/LCH/Blueprints/Effect/NS_Energy.NS_Energy" (`KismetMathLibrary.MakeVector` (.x BeamLocation) (.y BeamLocation)) (struct) (1.0 1.0 1.0) true true "AutoRelease"))
      (add `NiagaraComponent.OnSystemFinished` _returnvalue (delegate `OnSystemFinished`)))))

(event `OnSystemFinished`
  (params (PSystem :type "NiagaraComponent Object Reference"))
  ;[1 1 1] Beam Attack
  (bind _returnvalue (`KismetMathLibrary.MakeVector` (.x (stale `BeamAttack` BeamLocation)) (.y (stale `BeamAttack` BeamLocation))))
  (bind _returnvalue_2 (`NiagaraFunctionLibrary.SpawnSystemAtLocation` "/Game/LCH/Blueprints/Effect/NS_Beam.NS_Beam" _returnvalue (struct) (1.0 1.0 1.0) true true "AutoRelease"))
  (`NiagaraFunctionLibrary.SpawnSystemAtLocation` "/Game/LCH/Blueprints/Effect/NS_Shockwave.NS_Shockwave" _returnvalue (struct) (1.0 1.0 1.0) true true "AutoRelease")
  (add `NiagaraComponent.OnSystemFinished` _returnvalue_2 (delegate `OnSystemFinished_Event`)))

(event `OnSystemFinished_Event`
  (params (PSystem :type "NiagaraComponent Object Reference"))
  ;[1 1 1] Beam Attack
  (`KismetSystemLibrary.PrintString` "End!End!")
  (`self.OnAttackEnd`))

(event `SpawnMonsterAttack`
  (bind (_returnvalue_x _returnvalue_y _returnvalue_z) (`KismetMathLibrary.BreakVector` (`self.K2_GetActorLocation`)))
  ;[1 1 1] Monster Spawn Attack
  (`|PlayMontage` (`self.Mesh`) "/Game/LCH/Blueprints/Character/Tiger/Animations/ANIM_Lion_Roar_Montage.ANIM_Lion_Roar_Montage"
    (:`then`
      (`|SpawnActorFromClass` "/Game/LCU/Blueprints/Character/AI/BP_LCU_NormalMonster.BP_LCU_NormalMonster_C" (`KismetMathLibrary.MakeTransform` (`KismetMathLibrary.MakeVector` (+ _returnvalue_x (`KismetMathLibrary.RandomFloatInRange` 200.0 400.0)) (+ _returnvalue_y (`KismetMathLibrary.RandomFloatInRange` 200.0 400.0)) _returnvalue_z)) "AdjustIfPossibleButAlwaysSpawn" "MultiplyWithRoot" null null))
    (:`OnCompleted`
      (`self.OnAttackEnd` :!label _label))
    (:`OnBlendOut`
      (goto _label))
    (:`OnInterrupted`
      (goto _label))))

(event `FireBallAttack`
  (params (TargetActor :type "Actor Object Reference"))
  ;[1 1 1] FireBall Attack
  (`|PlayMontage` (`self.Mesh`) "/Game/LCH/Blueprints/Character/Tiger/Animations/ANIM_Lion_Roar_Montage.ANIM_Lion_Roar_Montage"
    (:`then`
      (`|SpawnActorFromClass` "/Game/LCH/Blueprints/Effect/BP_FireBallProjectile.BP_FireBallProjectile_C" (`KismetMathLibrary.MakeTransform` (`self.K2_GetActorLocation`)) "AlwaysSpawn" "MultiplyWithRoot" null null))))

(event `/Game/LCH/Blueprints/PhysicalAnimation/BPI_PhysicalAnimationable.PhysicalAnimate`
  (params (HitResult :type "HitResult Structure") (Power :type "Float (double-precision)"))
  (`/Game/LCH/Blueprints/PhysicalAnimation/PhysicalAnimComp.HitReaction` (`self.PhysicalAnimComp`) HitResult Power true))

(event `self.ReceiveAnyDamage`
  (params (Damage :type "Float (single-precision)") (DamageType :type "DamageType Object Reference") (InstigatedBy :type "Controller Object Reference") (DamageCauser :type "Actor Object Reference")))

(fn `GetPatrolSpline`
  (returns (PatrolSpline :type "/Game/LCH/Blueprints/Character/Tiger/AI/LCH_BP_Patrol Object Reference"))
  (return (`self.PatrolSpline`)))

(fn `SetMovementSpeed`
  (params (Speed :type "/Game/LCH/Blueprints/Character/Tiger/AI/LCH_E_MovementSpeed Enum" :default "NewEnumerator0"))
  (returns (SpeedValue :type "Float (double-precision)"))
  (bind _output_get (set `CharacterMovementComponent.MaxWalkSpeed` (select `/Game/LCH/Blueprints/Character/Tiger/AI/LCH_E_MovementSpeed` Speed :`NewEnumerator1` 300.0 :`NewEnumerator2` 500.0) (`self.CharacterMovement`)))
  (return _output_get))

(fn `UserConstructionScript`)