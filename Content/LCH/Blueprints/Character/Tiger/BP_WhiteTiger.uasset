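; BP_WhiteTiger is a tiger AI pawn that chases the player and performs a phantom-charge attack.
; FollowPlayer moves it to the player, calls Attack1 on arrival, then repeats after a delay.
; Attack1 spawns a collision-free copy of its own class behind and below it while playing an attack montage.
; A timeline drives the copy forward and animates its dynamic material's opacity until montage completion destroys it.
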(event `self.ReceiveBeginPlay`
  (`self.FollowPlayer`))

(event `self.ReceiveTick`
  (params (DeltaSeconds :type "Float (single-precision)")))

(event `FollowPlayer`
  (`|AIMoveTo` self (0.0 0.0 0.0) (`GameplayStatics.GetPlayerPawn` 0) 100.0
    (:`OnSuccess`
      (`KismetSystemLibrary.PrintString` "Hello")
      (`self.Attack1`)
      (`KismetSystemLibrary.Delay` 2.0)
      (`self.FollowPlayer`))))

(event `Attack1`
  (bind _returnvalue (`|SpawnActorFromClass` "BP_WhiteTiger_C" (`KismetMathLibrary.MakeTransform` (- (- (`self.K2_GetActorLocation`) (* (`self.GetActorForwardVector`) 200.0)) (* (`self.GetActorUpVector`) 200.0)) (`self.K2_GetActorRotation`)) "AdjustIfPossibleButAlwaysSpawn" "MultiplyWithRoot" self null))
  (bind _capsulecomponent (`Character.CapsuleComponent` _returnvalue))
  (`PrimitiveComponent.SetSimulatePhysics` _capsulecomponent false)
  (`PrimitiveComponent.SetCollisionEnabled` _capsulecomponent "NoCollision")
  (bind _returnvalue_2 (`PrimitiveComponent.CreateDynamicMaterialInstance` (`Character.Mesh` _returnvalue) 0 "/Game/LCH/Blueprints/Character/Tiger/Materials/M_WhiteTiger.M_WhiteTiger" "None"))
  (`self.PlayAnimMontage` _returnvalue null 1.0 "None")
  (`|PlayMontage` (`self.Mesh`) "/Game/LCH/Blueprints/Character/Cats/Animations/AM_Anim_CatStray_Attack_F.AM_Anim_CatStray_Attack_F"
    (:`then`
      (bind (_direction _speed _opacity) (`Timeline|Timeline` :!via `PlayFromStart`)
        (:`Update`
          (`/Engine/EditorBlueprintResources/StandardMacros.IsValid` _returnvalue
            (:`Is Valid`
              (`self.K2_SetActorLocation` _returnvalue (+ (`self.K2_GetActorLocation` _returnvalue) (* (`self.GetActorForwardVector` _returnvalue) (* (`KismetMathLibrary.Lerp` 0.0 1000.0 _speed) (`GameplayStatics.GetWorldDeltaSeconds`)))) false false)
              (`MaterialInstanceDynamic.SetScalarParameterValue` _returnvalue_2 "OpacityMultiply" (`KismetMathLibrary.Lerp` 0.0 1.0 _opacity)))))))
    (:`OnCompleted`
      (`self.K2_DestroyActor` _returnvalue))))

(fn `UserConstructionScript`)