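; Child sword Blueprint that triggers physical-animation hit reactions on BP_BlackTiger, with debug drawing and printing.
; Each Tick line-traces from the mesh's TraceSocket to a scaled down vector used as a world position, not a socket offset, skipping the last traced actor.
; Capsule overlaps also pass their sweep result to the tiger's HitReaction, without that repeat guard.
; Both paths supply fixed spine bone names.
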(event `self.ReceiveTick`
  (params (DeltaSeconds :type "Float (single-precision)"))
  (`parent.ReceiveTick` DeltaSeconds)
  (bind _outhit (`KismetSystemLibrary.LineTraceSingle` :`Start` (`SceneComponent.GetSocketLocation` (`self.StaticMesh`) "TraceSocket") :`End` (* (`KismetMathLibrary.Normal` (* (`self.GetActorUpVector`) -1.0)) 1000.0) :`TraceChannel` "TraceTypeQuery3" :`DrawDebugType` "ForDuration" :`DrawTime` 0.5))
  (bind (_bblockinghit _binitialoverlap _time _distance _location _impactpoint _normal _impactnormal _physmat _hitactor _hitcomponent _hitbonename) (`GameplayStatics.BreakHitResult` _outhit))
  (if (not (== (`self.LastTracedActor`) _hitactor))
    (bind _asbp_black_tiger (cast `/Game/LCH/Blueprints/Character/BP_BlackTiger` _hitactor)
      (:`then`
        (set `self.LastTracedActor` _asbp_black_tiger)
        (`/Game/LCH/Blueprints/PhysicalAnimation/PhysicalAnimComp_Tiger.HitReaction` (`/Game/LCH/Blueprints/Character/BP_BlackTiger.PhysicalAnimComp_Tiger` _asbp_black_tiger) _outhit "c_spine_01_uJnt_114" "c_spine_00_uJnt_115")
        (`KismetSystemLibrary.PrintString` (`KismetStringLibrary.Conv_NameToString` _hitbonename)))
      (:`CastFailed`
        (set `self.LastTracedActor` null)))))

(event `self.CapsuleCollision.OnComponentHit`
  (params (HitComponent :type "PrimitiveComponent Object Reference") (OtherActor :type "Actor Object Reference") (OtherComp :type "PrimitiveComponent Object Reference") (NormalImpulse :type "Vector Structure") (Hit :type "HitResult Structure (by ref)")))

(event `self.CapsuleCollision.OnComponentBeginOverlap`
  (params (OverlappedComponent :type "PrimitiveComponent Object Reference") (OtherActor :type "Actor Object Reference") (OtherComp :type "PrimitiveComponent Object Reference") (OtherBodyIndex :type Integer) (bFromSweep :type Boolean) (SweepResult :type "HitResult Structure (by ref)"))
  (bind (_bblockinghit _binitialoverlap _time _distance _location _impactpoint _normal _impactnormal _physmat _hitactor _hitcomponent _hitbonename _bonename _hititem _elementindex _faceindex _tracestart _traceend) (`GameplayStatics.BreakHitResult` SweepResult))
  (`KismetSystemLibrary.PrintString` (`KismetSystemLibrary.GetDisplayName` OtherActor))
  (bind _asbp_black_tiger (cast `/Game/LCH/Blueprints/Character/BP_BlackTiger` OtherActor))
  (`KismetSystemLibrary.PrintString` (`KismetStringLibrary.Conv_BoolToString` _bblockinghit))
  (`KismetSystemLibrary.DrawDebugSphere` _impactpoint 30.0 12 (struct :`R` 0.131597 :`B` 1.0 :`A` 1.0) 1.0 1.0)
  (`KismetSystemLibrary.DrawDebugLine` _tracestart _traceend (struct :`R` 1.0 :`B` 0.084735 :`A` 1.0) 1.0 1.0)
  (`/Game/LCH/Blueprints/PhysicalAnimation/PhysicalAnimComp_Tiger.HitReaction` (`/Game/LCH/Blueprints/Character/BP_BlackTiger.PhysicalAnimComp_Tiger` _asbp_black_tiger) SweepResult "c_spine_01_uJnt_114" "c_spine_00_uJnt_115"))

(fn `UserConstructionScript`
  (`parent.UserConstructionScript`))