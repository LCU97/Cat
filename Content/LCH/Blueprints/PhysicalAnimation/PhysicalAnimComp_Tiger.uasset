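; Physical animation component for BP_BlackTiger that adds physics-driven hit reactions to its skeletal mesh.
; HitReaction applies the "Tiger" profile, simulates bodies below a base bone, and shoves a fixed head bone along the trace direction, regardless of hit bone.
; Tick fades the physics blend weight from a fixed spine bone, then stops simulation and itself.
; TogglePhysicalAnimation separately enables half-blended simulation below given bones.
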(event `self.ReceiveBeginPlay`
  ;[1 1 1] Add 'Physical Animation Component' to Owner Actor and set Skeletal Mesh Component.
  (bind _returnvalue (`|AddComponentByClass` (`self.GetOwner`) "/Script/Engine.PhysicalAnimationComponent"))
  (bind _output_get (set `self.PhysicalAnimationComponent` _returnvalue))
  (bind _asbp_black_tiger (cast `/Game/LCH/Blueprints/Character/BP_BlackTiger` (`self.GetOwner`)))
  (bind _mesh (`Character.Mesh` _asbp_black_tiger))
  (`PhysicalAnimationComponent.SetSkeletalMeshComponent` _output_get _mesh)
  (set `self.Mesh` _mesh))

(event `TogglePhysicalAnimation`
  (params (BoneNames :type "Array of Name"))
  (bind _output_get (set `self.BoneNames` BoneNames))
  (for _array_element _output_get
    (`SkeletalMeshComponent.SetAllBodiesBelowSimulatePhysics` (`self.Mesh`) _array_element true true)
    (`SkeletalMeshComponent.SetAllBodiesBelowPhysicsBlendWeight` (`self.Mesh`) _array_element 0.5 false true)))

(event `HitReaction`
  (params (Hit :type "HitResult Structure") (SubstituteBoneName :type Name) (BaseBoneName :type Name))
  (bind (_bblockinghit _binitialoverlap _time _distance _location _impactpoint _normal _impactnormal _physmat _hitactor _hitcomponent _hitbonename _bonename _hititem _elementindex _faceindex _tracestart _traceend) (`GameplayStatics.BreakHitResult` Hit))
  ;[1 1 1] Hit Reaction (Add Impulse to hitted bone)
  (set `self.SubstituteBoneName` SubstituteBoneName)
  (`self.SetComponentTickEnabled` true)
  (set `self.HitReactionTimeRemaining` 1.0)
  (`PhysicalAnimationComponent.ApplyPhysicalAnimationProfileBelow` (`self.PhysicalAnimationComponent`) BaseBoneName "Tiger" false false)
  (`SkeletalMeshComponent.SetAllBodiesBelowSimulatePhysics` (`self.Mesh`) BaseBoneName true false)
  (`PrimitiveComponent.AddImpulse` (`self.Mesh`) (* (`KismetMathLibrary.Normal` (- _traceend _tracestart)) 8000.0) "c_head_00_uJnt_105" true))

(event `self.ReceiveTick`
  (params (DeltaSeconds :type "Float (single-precision)"))
  (set `self.HitReactionTimeRemaining` (- (`KismetMathLibrary.FInterpTo` (`self.HitReactionTimeRemaining`) 0.0 0.0 1.0) (* DeltaSeconds 1.5)))
  (if (<= (`self.HitReactionTimeRemaining`) 0.0)
    (set `self.HitReactionTimeRemaining` 0.0)
    (`SkeletalMeshComponent.SetAllBodiesBelowSimulatePhysics` (`self.Mesh`) "c_spine_00_uJnt_115" false true)
    (`self.SetComponentTickEnabled` false)
    (else
      (`SkeletalMeshComponent.SetAllBodiesBelowPhysicsBlendWeight` (`self.Mesh`) "c_spine_00_uJnt_115" (`KismetMathLibrary.FMin` (`self.HitReactionTimeRemaining`) 1.0) false true))))